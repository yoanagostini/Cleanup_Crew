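; Main menu player controller that puts the main menu widget on screen when play begins.
; BeginPlay creates WB_MainMenu, stores it, adds it to the viewport and switches input to UI-only with that widget focused.
; After a short delay it gives keyboard focus to the widget's Create Game button.
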(event `self.ReceiveBeginPlay`
  (bind _returnvalue (`|CreateWidget` "/Game/Game/Widgets/MainMenu/WB_MainMenu.WB_MainMenu_C" self))
  (bind _output_get (set `self.WB_MainMenu` _returnvalue))
  (`UserWidget.AddToViewport` _output_get 0)
  (`WidgetBlueprintLibrary.SetInputMode_UIOnlyEx` self (`self.WB_MainMenu`))
  (`KismetSystemLibrary.Delay` 0.2)
  (`Widget.SetKeyboardFocus` (`/Game/Game/Widgets/MainMenu/WB_MainMenu.CreateGame_Button` (`self.WB_MainMenu`))))

(fn `UserConstructionScript`)