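; Player character that moves and paints onto cleanable meshes beneath it.
; The movement input action feeds its 2D value directly into world-space X/Y movement, independent of facing.
; The interaction action runs a short downward complex line trace from the Cube component.
; If the hit actor is a BP_CleaningMech, it passes the collision UV to that actor's Draw function.
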(event `self.ReceiveBeginPlay`)

(event `EnhancedInput|/Game/Game/Inputs/AI_Movement`
  (params (ActionValue :type "Vector2D Structure") (ElapsedSeconds :type "Float (double-precision)") (TriggeredSeconds :type "Float (double-precision)") (InputAction :type "InputAction Object Reference" :default "/Game/Game/Inputs/AI_Movement.AI_Movement"))
  (:`Triggered`
    (`self.AddMovementInput` (`KismetMathLibrary.Conv_Vector2DToVector` ActionValue))))

(event `EnhancedInput|/Game/Game/Inputs/AI_Interactions`
  (params (ActionValue :type Boolean) (ElapsedSeconds :type "Float (double-precision)") (TriggeredSeconds :type "Float (double-precision)") (InputAction :type "InputAction Object Reference" :default "/Game/Game/Inputs/AI_Interactions.AI_Interactions"))
  (bind _returnvalue (`SceneComponent.K2_GetComponentLocation` (`self.Cube`)))
  (:`Triggered`
    (bind (_outhit _returnvalue_2) (`KismetSystemLibrary.LineTraceSingle` _returnvalue (- _returnvalue (0.0 0.0 100.0)) "TraceTypeQuery1" true))
    (if _returnvalue_2
      (bind _asbp_cleaning_mech (cast `/Game/Game/BP/Cleaning/BP_CleaningMech` (`.HitActor` (`GameplayStatics.BreakHitResult` _outhit))))
      (`/Game/Game/BP/Cleaning/BP_CleaningMech.Draw` _asbp_cleaning_mech (`GameplayStatics.FindCollisionUV` _outhit)))))

(fn `UserConstructionScript`)