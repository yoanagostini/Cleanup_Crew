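; Player controller that sets up input, a fixed camera view and a toggleable in-game menu.
; On BeginPlay it sets game-only input, then for the local controller adds the Enhanced Input mapping context and, after a short delay, spawns a camera at a fixed transform as the view target.
; The menu action lazily creates the widget, then toggles its visibility, switching cursor and input mode between game and UI.
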(event `self.ReceiveBeginPlay`
  (`WidgetBlueprintLibrary.SetInputMode_GameOnly` self)
  (if (`self.IsLocalController`)
    (`EnhancedInputSubsystemInterface.AddMappingContext` (pcsubsystem `EnhancedInputLocalPlayerSubsystem` self) "/Game/Game/Inputs/IMC_Player.IMC_Player" 0 (struct))
    (`KismetSystemLibrary.Delay` 1.0)
    (bind _returnvalue (`|SpawnActorFromClass` "/Script/Engine.CameraActor" (`KismetMathLibrary.MakeTransform` (-290.0 120.0 640.0) (struct :`Pitch` -45.0)) "Undefined" "MultiplyWithRoot" null null))
    (bind _output_get (set `self.CamRef` _returnvalue))
    (`self.SetViewTargetWithBlend` _output_get)))

(event `EnhancedInput|/Game/Game/Inputs/AI_GameMenu`
  (params (ActionValue :type Boolean) (ElapsedSeconds :type "Float (double-precision)") (TriggeredSeconds :type "Float (double-precision)") (InputAction :type "InputAction Object Reference" :default "/Game/Game/Inputs/AI_GameMenu.AI_GameMenu"))
  (:`Triggered`
    (`self.Toggle_GameMenu`)))

(fn `FocusGame`
  (set `self.bShowMouseCursor` false)
  (`WidgetBlueprintLibrary.SetInputMode_GameOnly` self))

(fn `FocusWidget`
  (set `self.bShowMouseCursor` true)
  (`WidgetBlueprintLibrary.SetInputMode_GameAndUIEx` self (`self.WB_GameMenu`)))

(fn `Toggle_GameMenu`
  (bind _wb_gamemenu (`self.WB_GameMenu`))
  (`self.WB_GameMenu`
    (:`then`
      (if (`Widget.IsVisible` _wb_gamemenu)
        (`Widget.SetVisibility` _wb_gamemenu "Collapsed")
        (`self.FocusGame`)
        (else
          (`Widget.SetVisibility` _wb_gamemenu "Visible")
          (`self.FocusWidget`))))
    (:`else`
      (bind _returnvalue (`|CreateWidget` "/Game/Game/Widgets/GameWidgets/WB_GameMenu.WB_GameMenu_C" self))
      (bind _output_get (set `self.WB_GameMenu` _returnvalue))
      (`UserWidget.AddToViewport` (`self.WB_GameMenu`) 0)
      (`UserWidget.AddToViewport` _output_get 0)
      (`self.FocusWidget`))))

(fn `UserConstructionScript`)