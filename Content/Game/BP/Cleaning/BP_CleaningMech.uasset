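; Cleaning-mechanic Blueprint that uses render-target masks for blood on Floor1, with a brush for painting into them.
; BeginPlay clears two targets, gives the floor a dynamic blood material using a random array target, and stamps blood spots onto RT_BloodMaskRender.
; Draw sets the brush's position and renders it into a randomly re-picked target, not necessarily the floor's.
; An editor-only call also snapshots a random target to a static texture, used only for debug printing.
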(event `self.ReceiveBeginPlay`
  (bind _rendertarget (`self.RenderTarget`))
  (bind _output (`|GetArrayItem` _rendertarget (`KismetMathLibrary.RandomInteger` (`KismetArrayLibrary.Array_Length` _rendertarget))))
  (bind _returnvalue (`KismetMaterialLibrary.CreateDynamicMaterialInstance` "/Game/Game/Materials/M_Brush_Inst.M_Brush_Inst"))
  (set `self.BrushRef` _returnvalue)
  (`self.ClearRenderTargets`)
  (bind _returnvalue_2 (`KismetRenderingLibrary.RenderTargetCreateStaticTexture2DEditorOnly` _output (`KismetStringLibrary.Conv_ObjectToString` _output)))
  (bind _output_get (set `self.RendTarg` _returnvalue_2))
  (`KismetSystemLibrary.PrintString` (`KismetSystemLibrary.GetDisplayName` _output_get))
  (bind _returnvalue_3 (`PrimitiveComponent.CreateDynamicMaterialInstance` (`self.Floor1`) 0 "/Game/Game/Materials/M_Blood_Inst.M_Blood_Inst" "None"))
  (`MaterialInstanceDynamic.SetTextureParameterValue` _returnvalue_3 "Param" _output)
  (`self.DrawBloodOnRenderTargets`))

(event `Draw`
  (params (Pos :type "Vector2D Structure"))
  (bind _rendertarget (`self.RenderTarget`))
  (`MaterialInstanceDynamic.SetVectorParameterValue` (`self.BrushRef`) "Pos" (`KismetMathLibrary.Conv_VectorToLinearColor` (`KismetMathLibrary.Conv_Vector2DToVector` Pos)))
  (`KismetRenderingLibrary.DrawMaterialToRenderTarget` (`|GetArrayItem` _rendertarget (`KismetMathLibrary.RandomInteger` (`KismetArrayLibrary.Array_Length` _rendertarget))) (`self.BrushRef`)))

(fn `ClearRenderTargets`
  (`|ExecutionSequence`
    (:`then_0`
      (`KismetRenderingLibrary.ClearRenderTarget2D` "/Game/Game/Materials/RT_BloodMaskRender.RT_BloodMaskRender"))
    (:`then_1`
      (`KismetRenderingLibrary.ClearRenderTarget2D` "/Game/Game/Materials/NewTextureRenderTarget2D.NewTextureRenderTarget2D"))))

(fn `DrawBloodOnRenderTargets`
  (`|ExecutionSequence`
    (:`then_0`
      (`KismetRenderingLibrary.DrawMaterialToRenderTarget` "/Game/Game/Materials/RT_BloodMaskRender.RT_BloodMaskRender" "/Game/Game/Materials/M_BloodSpots.M_BloodSpots"))))

(fn `UserConstructionScript`)